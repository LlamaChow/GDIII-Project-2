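; AI enemy that chases one of two players and deals damage on arrival.
; On BeginPlay it randomly picks player character 0 or 1, casts it to BP_ThirdPersonCharacterSynty and pursues it with AIMoveTo.
; Each successful move damages player 0, whichever target was picked, then repeats the chase on the same target after a short delay.
; A failed cast or move ends the loop.
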(event `self.ReceiveBeginPlay`
  (bind _output_get (set `self.Player Array` (`|MakeArray` (`GameplayStatics.GetPlayerCharacter` 0) (`GameplayStatics.GetPlayerCharacter` 1))))
  (bind _output_get_2 (set `self.selectedPlayer` (`KismetArrayLibrary.Array_Random` _output_get)))
  (bind _asbp_third_person_character_synty (cast `/Game/ThirdPerson/Blueprints/BP_ThirdPersonCharacterSynty` _output_get_2 :!label _label))
  (`|AIMoveTo` self (0.0 0.0 0.0) _asbp_third_person_character_synty
    (:`OnSuccess`
      (`GameplayStatics.ApplyDamage` (`GameplayStatics.GetPlayerCharacter` 0) 1.0)
      (`KismetSystemLibrary.Delay` 1.0)
      (goto _label))))

(fn `UserConstructionScript`)
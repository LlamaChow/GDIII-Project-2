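; AI enemy pawn that ragdolls its mesh when health runs out, then destroys itself five seconds later, checked on Tick.
; Chase logic picks a random player, follows with AIMoveTo, then repeatedly damages player 0 on arrival, regardless of target.
; That chase logic, along with health and player-array setup, is disconnected from the empty BeginPlay, so it never runs.
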(event `self.ReceiveBeginPlay`)

(event `self.ReceiveTick`
  (params (DeltaSeconds :type "Float (single-precision)"))
  ;[1 1 1] When an enemy dies, they collapse and disappear after a few seconds.
  (if (<= (`self.health`) 0.0)
    (`PrimitiveComponent.SetSimulatePhysics` (`self.Mesh`) true)
    (`KismetSystemLibrary.Delay` 5.0)
    (`self.K2_DestroyActor`)))

(fn `UserConstructionScript`)
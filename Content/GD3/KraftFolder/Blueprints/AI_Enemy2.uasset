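; AI_Enemy2 is an enemy that chases a player, deals periodic damage and ragdolls on death.
; BeginPlay sets Health, inserts player 0 into PlayerArray and picks a random entry to pursue; the gathered ClassActors list goes unused.
; Each successful AIMoveTo damages player 0 regardless of target, then loops after a delay.
; Tick polls Health, enabling mesh physics and destroying the actor after a delay once it reaches zero.
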(event `self.ReceiveBeginPlay`
  (`|ExecutionSequence`
    (:`then_0`
      (set `self.health` 1000.0))
    (:`then_1`
      (`KismetArrayLibrary.Array_Insert` (`self.Player Array`) (`GameplayStatics.GetPlayerCharacter` 0))
      (bind _outactors (`GameplayStatics.GetAllActorsOfClass` "/Game/ThirdPerson/Blueprints/BP_ThirdPersonCharacterSynty.BP_ThirdPersonCharacterSynty_C"))
      (set `self.classActors` _outactors))
    (:`then_2`
      ;[1 1 1] Enemies randomly choose a player to pursue.
      (bind _output_get (set `self.Player Array` (`self.Player Array`)))
      (bind _output_get_2 (set `self.selectedPlayer` (`KismetArrayLibrary.Array_Random` _output_get))) ; Stores the random index as a constant variable for the enemy to chase.
      (bind _asbp_third_person_character_synty (cast `/Game/ThirdPerson/Blueprints/BP_ThirdPersonCharacterSynty` _output_get_2 :!label _label))
      (`|AIMoveTo` self (0.0 0.0 0.0) _asbp_third_person_character_synty
        (:`OnSuccess`
          ;[1 1 1] When enemies reach a player, they apply one damage per (x) seconds. If the player leaves the acceptance radius, the chase resumes.
          (`GameplayStatics.ApplyDamage` (`GameplayStatics.GetPlayerCharacter` 0) 1.0)
          (`KismetSystemLibrary.Delay` 1.5)
          (goto _label))))))

(event `self.ReceiveTick`
  (params (DeltaSeconds :type "Float (single-precision)"))
  ;[1 1 1] When an enemy dies, they collapse and disappear after a few seconds.
  (if (<= (`self.health`) 0.0)
    (`PrimitiveComponent.SetSimulatePhysics` (`self.Mesh`) true)
    (`KismetSystemLibrary.Delay` 5.0)
    (`self.K2_DestroyActor`)))

(fn `UserConstructionScript`)
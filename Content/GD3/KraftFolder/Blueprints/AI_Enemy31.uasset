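; Enemy AI that picks a random BP_ThirdPersonCharacterSynty on spawn and chases it with AIMoveTo.
; On each arrival it waits, applies damage to the character at PlayerIndex rather than the chased reference, then resumes the chase.
; Tick triggers death (ragdoll, delayed destroy) at zero Health.
; Tick also drives a location-comparison stall check that clears IsMoving, though its EnemyDeath call only acts if IsDead is set.
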(event `self.ReceiveBeginPlay`
  (`|ExecutionSequence`
    (:`then_0`
      (set `self.health` 1000.0)
      (`KismetSystemLibrary.Delay` 0.2))
    (:`then_1`
      (for _index (range 2)
        (bind _outactors (`GameplayStatics.GetAllActorsOfClass` "/Game/ThirdPerson/Blueprints/BP_ThirdPersonCharacterSynty.BP_ThirdPersonCharacterSynty_C"))
        (bind _output_get (set `self.PlayerArray` _outactors))
        (`KismetArrayLibrary.Array_Insert` _output_get null _index)
        (`/Engine/EditorBlueprintResources/StandardMacros.IncrementInt` _index))
      ;[1 1 1] Enemies randomly choose a player to pursue.
      (bind _output_get_2 (set `self.PlayerArray` (`self.PlayerArray`)))
      (bind _output_get_3 (set `self.selectedPlayer` (`KismetArrayLibrary.Array_Random` _output_get_2))) ; Stores the random index as a constant variable for the enemy to chase.
      (bind _asbp_third_person_character_synty (cast `/Game/ThirdPerson/Blueprints/BP_ThirdPersonCharacterSynty` _output_get_3 :!label _label))
      (set `self.isDealingDamage?` false)
      (set `self.isMoving?` true)
      (`|AIMoveTo` self (0.0 0.0 0.0) _asbp_third_person_character_synty
        (:`OnSuccess`
          ;[1 1 1] When enemies reach a player, they apply one damage per (x) seconds. If the player leaves the acceptance radius, the chase resumes.
          (`KismetSystemLibrary.Delay` 1.5) ; (x) seconds
          (set `self.isDealingDamage?` true)
          (`GameplayStatics.ApplyDamage` (`GameplayStatics.GetPlayerCharacter` (`self.playerIndex`)) 1.0)
          (goto _label))))))

(event `self.ReceiveTick`
  (params (DeltaSeconds :type "Float (single-precision)"))
  (`|ExecutionSequence`
    (:`then_0`
      (if (<= (`self.health`) 0.0)
        (set `self.isDead?` true)
        (`self.EnemyDeath`)))
    (:`then_1`
      (`/Engine/EditorBlueprintResources/StandardMacros.DoOnce` false :!label _label_2
        (:`Completed`
          (`self.WorldLocationUpdate`))))
    (:`then_2`
      (if (`self.isMoving?`)
        (goto _label_2 :!via `Reset`)))))

(event `EnemyDeath`
  ;[1 1 1] When an enemy dies, they collapse and disappear after a few seconds.
  (if (`self.isDead?`)
    (`PrimitiveComponent.SetSimulatePhysics` (`self.Mesh`) true)
    (`KismetSystemLibrary.Delay` 5.0)
    (`self.K2_DestroyActor`)))

(event `WorldLocationUpdate`
  (set `self.worldLocation` (`SceneComponent.K2_GetComponentLocation` (`self.Mesh`)))
  (`self.AILocationCompare`)
  (if (`self.isDealingDamage?`)
    _
    (elif (not (`self.isMoving?`))
      (`self.EnemyDeath`))))

(fn `UserConstructionScript`)
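; AI_Enemy3 is an enemy that chases a player and deals repeated damage on reaching its target.
; BeginPlay sets up health and picks randomly from PlayerArray, which receives only player 0, then loops AIMoveTo, damage to player 0 and a delay.
; An overlap range toggles its health widget for player characters.
; Tick ragdolls and later destroys it when MaxHealth, not CurrentHealth, reaches zero; no damage handling exists here.
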(event `self.WidgetRange.OnComponentBeginOverlap`
  (params (OverlappedComponent :type "PrimitiveComponent Object Reference") (OtherActor :type "Actor Object Reference") (OtherComp :type "PrimitiveComponent Object Reference") (OtherBodyIndex :type Integer) (bFromSweep :type Boolean) (SweepResult :type "HitResult Structure (by ref)"))
  (cast `/Game/ThirdPerson/Blueprints/BP_ThirdPersonCharacterSynty` OtherActor)
  (`SceneComponent.SetVisibility` (`self.Widget`) true false))

(event `self.WidgetRange.OnComponentEndOverlap`
  (params (OverlappedComponent :type "PrimitiveComponent Object Reference") (OtherActor :type "Actor Object Reference") (OtherComp :type "PrimitiveComponent Object Reference") (OtherBodyIndex :type Integer))
  (cast `/Game/ThirdPerson/Blueprints/BP_ThirdPersonCharacterSynty` OtherActor)
  (`SceneComponent.SetVisibility` (`self.Widget`) false false))

(event `self.ReceiveBeginPlay`
  (`|ExecutionSequence`
    (:`then_0`
      (bind _aswb_health (cast `/Game/GD3/Aj/Blueprints/WB_Health` (`WidgetComponent.GetUserWidgetObject` (`self.Widget`))))
      (bind _output_get (set `self.HealthWidget` _aswb_health))
      (`/Game/GD3/Aj/Blueprints/WB_Health.UpdateHealthUI` _output_get (stale _output_get_2) (stale _output_get_2)))
    (:`then_1`
      (bind _output_get_2 (set `self.MaxHealth` 1000.0))
      (set `self.CurrentHealth` _output_get_2))
    (:`then_2`
      (`KismetArrayLibrary.Array_Insert` (`self.PlayerArray`) (`GameplayStatics.GetPlayerCharacter` 0))
      (bind _outactors (`GameplayStatics.GetAllActorsOfClass` "/Game/ThirdPerson/Blueprints/BP_ThirdPersonCharacterSynty.BP_ThirdPersonCharacterSynty_C"))
      (set `self.classActors` _outactors))
    (:`then_3`
      ;[1 1 1] Enemies randomly choose a player to pursue.
      (bind _output_get_3 (set `self.PlayerArray` (`self.PlayerArray`)))
      (bind _output_get_4 (set `self.selectedPlayer` (`KismetArrayLibrary.Array_Random` _output_get_3))) ; Stores the random index as a constant variable for the enemy to chase.
      (bind _asbp_third_person_character_synty (cast `/Game/ThirdPerson/Blueprints/BP_ThirdPersonCharacterSynty` _output_get_4 :!label _label))
      (`|AIMoveTo` self (0.0 0.0 0.0) _asbp_third_person_character_synty
        (:`OnSuccess`
          ;[1 1 1] When enemies reach a player, they apply one damage per second. If the player leaves the acceptance radius, the chase resumes.
          (`GameplayStatics.ApplyDamage` (`GameplayStatics.GetPlayerCharacter` 0) 1.0)
          (`KismetSystemLibrary.Delay` 1.0)
          (goto _label))))))

(event `self.ReceiveTick`
  (params (DeltaSeconds :type "Float (single-precision)"))
  ;[1 1 1] When an enemy dies, they collapse and disappear after a few seconds.
  (if (<= (`self.MaxHealth`) 0.0)
    (`PrimitiveComponent.SetSimulatePhysics` (`self.Mesh`) true)
    (`KismetSystemLibrary.Delay` 5.0)
    (`self.K2_DestroyActor`)))

(fn `UserConstructionScript`)
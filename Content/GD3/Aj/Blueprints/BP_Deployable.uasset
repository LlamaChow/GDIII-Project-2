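; BP_Deployable is a thrown deployable actor with an area of effect, apparently a base or stub for effects on enemies.
; Throw sets and activates projectile movement with the given velocity, reveals the mesh after a short delay, then sets a brief lifespan.
; Overlaps with the AreaofEffect component call DeployableEffect, which checks for the Enemy tag but applies nothing yet.
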(event `self.AreaofEffect.OnComponentBeginOverlap`
  (params (OverlappedComponent :type "PrimitiveComponent Object Reference") (OtherActor :type "Actor Object Reference") (OtherComp :type "PrimitiveComponent Object Reference") (OtherBodyIndex :type Integer) (bFromSweep :type Boolean) (SweepResult :type "HitResult Structure (by ref)"))
  (`self.DeployableEffect`))

(event `DeployableEffect`
  (if (`self.ActorHasTag` (stale `self.AreaofEffect.OnComponentBeginOverlap` OtherActor) "Enemy")
    _))

(event `Throw`
  (params (Velocity :type "Vector Structure"))
  (set `MovementComponent.Velocity` Velocity (`self.ProjectileMovement`))
  (`ActorComponent.Activate` (`self.ProjectileMovement`) false)
  (`KismetSystemLibrary.Delay` 0.4)
  (`SceneComponent.SetHiddenInGame` (`self.DeployableMesh`) false false)
  (`self.SetLifeSpan` 2.5))

(fn `UserConstructionScript`)